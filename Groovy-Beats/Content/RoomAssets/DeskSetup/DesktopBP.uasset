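; Desktop PC actor for the desk setup whose power button lets the VR player switch the computer on and off.
; Overlap events on PowerButton track whether the player, cached as the first VRPawn at BeginPlay, is in range.
; TriggerPressed flips the power state while in range, playing an on or off cue at the PC mesh and swapping the screen material on the referenced MonitorScreen.
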(event OnComponentBeginOverlap(PowerButton)
  (params (OverlappedComponent :type Primitive%20Component%20Object%20Reference) (OtherActor :type Actor%20Object%20Reference) (OtherComp :type Primitive%20Component%20Object%20Reference) (OtherBodyIndex :type Integer) (bFromSweep :type Boolean) (SweepResult :type Hit%20Result%20Structure%20%28by%20ref%29))
  (if (== OtherActor (Variables|Default|GetPlayer))
    (Variables|Default|SetisInteracting true)))

(event OnComponentEndOverlap(PowerButton)
  (params (OverlappedComponent :type Primitive%20Component%20Object%20Reference) (OtherActor :type Actor%20Object%20Reference) (OtherComp :type Primitive%20Component%20Object%20Reference) (OtherBodyIndex :type Integer))
  (if (== OtherActor (Variables|Default|GetPlayer))
    (Variables|Default|SetisInteracting false)))

(event Custom|PCPowerOn
  (Audio|PlaySoundatLocation "/Game/Sound/Desktops/PowerOnCue.PowerOnCue" (Transformation|GetWorldLocation (Variables|Default|GetDesktopPCMesh)) "0, 0, 0" 1.0 1.0 0.0 0 0 0)
  (Rendering|Material|SetMaterial (Variables|/Game/RoomAssets/DeskSetup/Monitor/MonitorBP.MonitorBP_C|GetMonitor (Variables|Default|GetMonitorScreen)) 1 "/Game/RoomAssets/DeskSetup/Monitor/MonitorMaterialScreenOn.MonitorMaterialScreenOn"))

(event Custom|PCPowerOff
  (Audio|PlaySoundatLocation "/Game/Sound/Desktops/PowerOffCue.PowerOffCue" (Transformation|GetWorldLocation (Variables|Default|GetDesktopPCMesh)) "0, 0, 0" 1.0 1.0 0.0 0 0 0)
  (Rendering|Material|SetMaterial (Variables|/Game/RoomAssets/DeskSetup/Monitor/MonitorBP.MonitorBP_C|GetMonitor (Variables|Default|GetMonitorScreen)) 1 "/Game/RoomAssets/DeskSetup/Monitor/MonitorMaterialScreenOff.MonitorMaterialScreenOff"))

(event EventTick
  (params (DeltaSeconds :type Float%20%28single-precision%29)))

(event EventBeginPlay
  (bind _outactors (Actor|GetAllActorsOfClass "/Game/VRTemplate/Blueprints/VRPawn.VRPawn_C"))
  (Variables|Default|SetPlayer (Utilities|Array|Get(acopy) _outactors))
  (Variables|Default|SetPowerStatus true))

(event EventTriggerPressed
  (if (Variables|Default|GetisInteracting)
    (bind _output_get (Variables|Default|SetPowerStatus (not (Variables|Default|GetPowerStatus))))
    (if _output_get
      (CallFunction|PCPoweron)
      (else
        (CallFunction|PCPowerOff)))))

(fn ConstructionScript)