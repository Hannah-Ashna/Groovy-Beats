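; MonitorBP is a breakable desk monitor that shatters when an actor implementing GrippableInterface overlaps its box collision.
; The overlap hides the intact mesh, then reveals four pre-cracked pieces and turns on their physics simulation as a simple mesh-swap fracture.
; After a short delay the whole actor destroys itself, removing the debris.
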(event OnComponentBeginOverlap(BoxCollision)
  (params (OverlappedComponent :type Primitive%20Component%20Object%20Reference) (OtherActor :type Actor%20Object%20Reference) (OtherComp :type Primitive%20Component%20Object%20Reference) (OtherBodyIndex :type Integer) (bFromSweep :type Boolean) (SweepResult :type Hit%20Result%20Structure%20%28by%20ref%29))
  (if (Utilities|DoesObjectImplementInterface OtherActor "/Game/TheMatrix/GrippableInterface.GrippableInterface_C")
    (Rendering|SetVisibility (Variables|Default|GetMonitorCracked_Monitor_Part_2) true false)
    (Physics|SetSimulatePhysics (Variables|Default|GetMonitorCracked_Monitor_Part_1) true)
    (Rendering|SetVisibility (Variables|Default|GetMonitor) false false)
    (Utilities|FlowControl|Delay 1.5)
    (Actor|DestroyActor)))

(fn ConstructionScript)