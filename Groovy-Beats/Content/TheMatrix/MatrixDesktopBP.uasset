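; Desktop PC actor for the VR Matrix game that, when shut down, heals the player and damages the BigEnemy, both cached on BeginPlay.
; A trigger press while the player overlaps the power button shuts it off once, playing a sound and blanking the linked monitor.
; A grippable object hitting it while powered also shuts it off, then swaps the mesh for physics-simulated cracked pieces and destroys the actor after a delay.
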(event OnComponentBeginOverlap(PowerButton)
  (params (OverlappedComponent :type Primitive%20Component%20Object%20Reference) (OtherActor :type Actor%20Object%20Reference) (OtherComp :type Primitive%20Component%20Object%20Reference) (OtherBodyIndex :type Integer) (bFromSweep :type Boolean) (SweepResult :type Hit%20Result%20Structure%20%28by%20ref%29))
  (if (== OtherActor (Variables|Default|GetPlayer))
    (Variables|Default|SetisInteracting true)))

(event OnComponentEndOverlap(PowerButton)
  (params (OverlappedComponent :type Primitive%20Component%20Object%20Reference) (OtherActor :type Actor%20Object%20Reference) (OtherComp :type Primitive%20Component%20Object%20Reference) (OtherBodyIndex :type Integer))
  (if (== OtherActor (Variables|Default|GetPlayer))
    (Variables|Default|SetisInteracting false)))

(event OnComponentBeginOverlap(DesktopCollision)
  (params (OverlappedComponent :type Primitive%20Component%20Object%20Reference) (OtherActor :type Actor%20Object%20Reference) (OtherComp :type Primitive%20Component%20Object%20Reference) (OtherBodyIndex :type Integer) (bFromSweep :type Boolean) (SweepResult :type Hit%20Result%20Structure%20%28by%20ref%29))
  (if (and (Utilities|DoesObjectImplementInterface OtherActor "/Game/TheMatrix/GrippableInterface.GrippableInterface_C") (Variables|Default|GetPowerStatus))
    (CallFunction|PCPowerOff)
    (CallFunction|DestroyPC)))

(event Custom|DestroyPC
  (bind _desktopcracked_box001_part_1 (Variables|Default|GetDesktopCracked_Box001_Part_1))
  (Rendering|SetVisibility _desktopcracked_box001_part_1 true false)
  (Physics|SetSimulatePhysics _desktopcracked_box001_part_1 true)
  (Rendering|SetVisibility (Variables|Default|GetDesktopMesh) false false)
  (Utilities|FlowControl|Delay 2.0)
  (Actor|DestroyActor))

(event Custom|PCPowerOff
  (bind _monitorscreen (Variables|Default|GetMonitorScreen))
  (Audio|PlaySoundatLocation "/Game/Sound/Desktops/MatrixShutdownSFX.MatrixShutdownSFX" (Transformation|GetWorldLocation (Variables|Default|GetDesktopMesh)) "0, 0, 0" 1.0 1.0 0.0 0 0 0)
  (Utilities|IsValid _monitorscreen
    (:Is%20Valid
      (Rendering|Material|SetMaterial (Variables|/Game/RoomAssets/DeskSetup/Monitor/MonitorBP.MonitorBP_C|GetMonitor _monitorscreen) 1 "/Game/RoomAssets/DeskSetup/Monitor/MonitorMaterialScreenOff.MonitorMaterialScreenOff"))
    (:Is%20Not%20Valid
      _))
  (Default|Heal (Variables|Default|GetPlayer) 25.0)
  (Default|TakeDamage (Variables|Default|GetBig%20Enemy) 2e+01)
  (Variables|Default|SetPowerStatus false))

(event EventBeginPlay
  (bind _outactors (Actor|GetAllActorsOfClass "/Game/TheMatrix/VRMatrixChar.VRMatrixChar_C"))
  (Variables|Default|SetPlayer (Utilities|Array|Get(acopy) _outactors))
  (bind _outactors_2 (Actor|GetAllActorsOfClass "/Game/TheMatrix/BigEnemy.BigEnemy_C"))
  (Variables|Default|SetBig%20Enemy (Utilities|Array|Get(acopy) _outactors_2))
  (Variables|Default|SetPowerStatus true))

(event EventTriggerPressed
  (if (and (Variables|Default|GetisInteracting) (Variables|Default|GetPowerStatus))
    (bind _output_get (Variables|Default|SetPowerStatus (not (Variables|Default|GetPowerStatus))))
    (if (not _output_get)
      (CallFunction|PCPowerOff))))

(fn ConstructionScript)