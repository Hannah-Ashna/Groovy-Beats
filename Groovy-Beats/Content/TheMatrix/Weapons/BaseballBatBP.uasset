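; BaseballBatBP is a grabbable baseball bat weapon for motion controllers that hurts patrolling minions.
; Grab attaches it to the passed motion controller and Release detaches the Sword component, both keeping world transforms.
; Sword overlaps deal fixed damage to PatrollingMinionAI actors with a hit sound.
; Overlaps with MatrixDesktopBP and MonitorBP props only play that sound.
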(event OnComponentBeginOverlap(Sword)
  (params (OverlappedComponent :type Primitive%20Component%20Object%20Reference) (OtherActor :type Actor%20Object%20Reference) (OtherComp :type Primitive%20Component%20Object%20Reference) (OtherBodyIndex :type Integer) (bFromSweep :type Boolean) (SweepResult :type Hit%20Result%20Structure%20%28by%20ref%29))
  (bind _returnvalue (Utilities|GetClass OtherActor))
  (bind _sword (Variables|Default|GetSword))
  (bind _returnvalue_2 (Transformation|GetWorldLocation _sword))
  (if (Utilities|ClassIsChildOf (Utilities|GetClass OtherActor) "/Game/TheMatrix/Enemies/EnemyAI/PatrollingMinionAI.PatrollingMinionAI_C")
    (bind _aspatrolling_minion_ai (Utilities|Casting|CastToPatrollingMinionAI OtherActor))
    (Default|TakeDamage _aspatrolling_minion_ai 4.0)
    (Audio|PlaySoundatLocation "/Game/Sound/BatHit_SoundCue.BatHit_SoundCue" _returnvalue_2 "0, 0, 0" 1.0 1.0 0.0 0 0 0)
    (elif (or (Utilities|ClassIsChildOf _returnvalue "/Game/TheMatrix/MatrixDesktopBP.MatrixDesktopBP_C") (Utilities|ClassIsChildOf _returnvalue "/Game/RoomAssets/DeskSetup/Monitor/MonitorBP.MonitorBP_C"))
      (Audio|PlaySoundatLocation "/Game/Sound/BatHit_SoundCue.BatHit_SoundCue" _returnvalue_2 "0, 0, 0" 1.0 1.0 0.0 0 0 0))))

(event EventGrab
  (params (Motion%20Controller :type Motion%20Controller%20Component%20Object%20Reference))
  (bind _output_get (Variables|Default|SetMotion%20Controller Motion%20Controller))
  (Transformation|AttachComponentToComponent _output_get "None" "KeepWorld" "KeepWorld" "KeepWorld" true))

(event EventRelease
  (params (Motion%20Controller :type Motion%20Controller%20Component%20Object%20Reference))
  (Utilities|IsValid (Variables|Default|GetMotion%20Controller)
    (:Is%20Valid
      (Transformation|DetachFromComponent (Variables|Default|GetSword) "KeepWorld" "KeepWorld" "KeepWorld" true))))

(fn ConstructionScript)