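; Melee enemy minion that hunts the VR player and punches them for damage.
; On BeginPlay it finds the VRMatrixChar, focuses its AI controller on it and chases it with a self-restarting AIMoveTo loop.
; An AttackRange overlap toggles the attack flags, which gate damage dealt by PunchCollision overlaps.
; TakeDamage lowers Health and prints debug text, while Tick polls for zero health to play a glitch sound and destroy the actor after a delay.
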(event OnComponentBeginOverlap(AttackRange)
  (params (OverlappedComponent :type Primitive%20Component%20Object%20Reference) (OtherActor :type Actor%20Object%20Reference) (OtherComp :type Primitive%20Component%20Object%20Reference) (OtherBodyIndex :type Integer) (bFromSweep :type Boolean) (SweepResult :type Hit%20Result%20Structure%20%28by%20ref%29))
  (if (and (== OtherActor (Variables|Default|GetPlayer)) (not (Variables|Default|GetIsAttacking)))
    (Variables|Default|SetCanAttack true)
    (Variables|Default|SetIsAttacking true)))

(event OnComponentEndOverlap(AttackRange)
  (params (OverlappedComponent :type Primitive%20Component%20Object%20Reference) (OtherActor :type Actor%20Object%20Reference) (OtherComp :type Primitive%20Component%20Object%20Reference) (OtherBodyIndex :type Integer))
  (if (and (== OtherActor (Variables|Default|GetPlayer)) (Variables|Default|GetCanAttack))
    (Variables|Default|SetCanAttack false)
    (Variables|Default|SetIsAttacking false)))

(event OnComponentBeginOverlap(PunchCollision)
  (params (OverlappedComponent :type Primitive%20Component%20Object%20Reference) (OtherActor :type Actor%20Object%20Reference) (OtherComp :type Primitive%20Component%20Object%20Reference) (OtherBodyIndex :type Integer) (bFromSweep :type Boolean) (SweepResult :type Hit%20Result%20Structure%20%28by%20ref%29))
  (bind _player (Variables|Default|GetPlayer))
  (if (and (== OtherActor _player) (Variables|Default|GetCanAttack))
    (Default|TakeDamage _player 2e+01)))

(event Custom|GetPlayer
  (Utilities|FlowControl|Delay 1.0)
  (bind _outactors (Actor|GetAllActorsOfClass "/Game/TheMatrix/VRMatrixChar.VRMatrixChar_C"))
  (bind _output_get (Variables|Default|SetPlayer (Utilities|Array|Get(acopy) _outactors)))
  (AI|SetFocus (Variables|Default|GetAI%20Controller) _output_get))

(event Custom|BaseMovement
  (bind _player (Variables|Default|GetPlayer))
  (Utilities|IsValid _player :!label _label
    (:Is%20Valid
      (AI|AIMoveTo self "0, 0, 0" _player 1e+01 true
        (:OnSuccess
          (Utilities|FlowControl|Delay 2.0)
          (goto _label))
        (:OnFail
          (goto _label))))
    (:Is%20Not%20Valid
      (Utilities|FlowControl|Delay 1.0)
      (goto _label))))

(event Custom|TakeDamage
  (params (Amount :type Float%20%28single-precision%29))
  (bind _output_get (Variables|Default|SetHealth (- (Variables|Default|GetHealth) Amount)))
  (if (> _output_get 0.0)
    (Development|PrintString (Utilities|String|ToString(Float) _output_get) true true "(R=1.000000,G=0.000000,B=0.014690,A=1.000000)" 4.0)
    (else
      (Development|PrintString "ENEMY DEAD" true true "(R=1.000000,G=0.000000,B=0.013544,A=1.000000)" 4.0))))

(event EventBeginPlay
  (Utilities|FlowControl|Sequence
    (:then_0
      (CallFunction|GetPlayer))
    (:then_1
      (CallFunction|BaseMovement))
    (:then_2
      (bind _asminion_aicontroller (Utilities|Casting|CastToMinion_AIController (Pawn|GetController)))
      (Variables|Default|SetAI%20Controller _asminion_aicontroller))))

(event EventTick
  (params (DeltaSeconds :type Float%20%28single-precision%29))
  (if (not (> (Variables|Default|GetHealth) 0.0))
    (Variables|Default|SetIsAttacking false)
    (Audio|PlaySoundatLocation "/Game/Sound/Enemies/GlitchDeath.GlitchDeath" (Transformation|GetWorldLocation (Variables|Collision|GetCapsuleComponent)) "0, 0, 0" 1.0 1.0 0.0 0 0 0)
    (Utilities|FlowControl|Delay 2.5)
    (Actor|DestroyActor)))

(fn ConstructionScript)