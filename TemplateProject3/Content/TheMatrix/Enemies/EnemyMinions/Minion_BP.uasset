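; Enemy minion that chases the VR player character and deals punch damage up close.
; On BeginPlay it caches its AI controller, finds the VRMatrixChar after a short delay and sets it as focus.
; A self-restarting AI Move To loop follows the player, pausing after each arrival.
; The AttackRange overlap toggles the attack flags, and PunchCollision overlaps apply fixed damage while attacking is allowed.
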(event OnComponentBeginOverlap(AttackRange)
  (params (OverlappedComponent :type Primitive%20Component%20Object%20Reference) (OtherActor :type Actor%20Object%20Reference) (OtherComp :type Primitive%20Component%20Object%20Reference) (OtherBodyIndex :type Integer) (bFromSweep :type Boolean) (SweepResult :type Hit%20Result%20Structure%20%28by%20ref%29))
  (if (and (== OtherActor (Variables|Default|GetPlayer)) (not (Variables|Default|GetIsAttacking)))
    (Variables|Default|SetCanAttack true)
    (Variables|Default|SetIsAttacking true)))

(event OnComponentEndOverlap(AttackRange)
  (params (OverlappedComponent :type Primitive%20Component%20Object%20Reference) (OtherActor :type Actor%20Object%20Reference) (OtherComp :type Primitive%20Component%20Object%20Reference) (OtherBodyIndex :type Integer))
  (if (and (== OtherActor (Variables|Default|GetPlayer)) (Variables|Default|GetCanAttack))
    (Variables|Default|SetCanAttack false)
    (Variables|Default|SetIsAttacking false)))

(event OnComponentBeginOverlap(PunchCollision)
  (params (OverlappedComponent :type Primitive%20Component%20Object%20Reference) (OtherActor :type Actor%20Object%20Reference) (OtherComp :type Primitive%20Component%20Object%20Reference) (OtherBodyIndex :type Integer) (bFromSweep :type Boolean) (SweepResult :type Hit%20Result%20Structure%20%28by%20ref%29))
  (bind _player (Variables|Default|GetPlayer))
  (if (and (== OtherActor _player) (Variables|Default|GetCanAttack))
    (Default|TakeDamage _player 2e+01)))

(event Custom|GetPlayer
  (Utilities|FlowControl|Delay 1.0)
  (bind _outactors (Actor|GetAllActorsOfClass "/Game/VRTemplate/Blueprints/VRMatrixChar.VRMatrixChar_C"))
  (bind _output_get (Variables|Default|SetPlayer (Utilities|Array|Get(acopy) _outactors)))
  (AI|SetFocus (Variables|Default|GetAI%20Controller) _output_get))

(event Custom|BaseMovement
  (bind _player (Variables|Default|GetPlayer))
  (Utilities|IsValid _player :!label _label
    (:Is%20Valid
      (AI|AIMoveTo self "0, 0, 0" _player 1e+01 true
        (:OnSuccess
          (Utilities|FlowControl|Delay 2.0)
          (goto _label))
        (:OnFail
          (goto _label))))
    (:Is%20Not%20Valid
      (Utilities|FlowControl|Delay 1.0)
      (goto _label))))

(event EventBeginPlay
  (Utilities|FlowControl|Sequence
    (:then_0
      (CallFunction|GetPlayer))
    (:then_1
      (CallFunction|BaseMovement))
    (:then_2
      (bind _asminion_aicontroller (Utilities|Casting|CastToMinion_AIController (Pawn|GetController)))
      (Variables|Default|SetAI%20Controller _asminion_aicontroller))))

(fn ConstructionScript)