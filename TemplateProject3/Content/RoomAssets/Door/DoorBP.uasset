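; DoorBP is a door that takes the VR pawn to MatrixLevel once its DoorOpen flag is set.
; While open, it raises its point light on Tick, and player overlap with the trigger plays a shutdown sound, then loads the level after a short delay.
; Handle overlaps track interaction so TriggerPressed plays a handle sound.
; DoorOpen starts false and nothing in this Blueprint sets it true.
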(event OnComponentBeginOverlap(Trigger)
  (params (OverlappedComponent :type Primitive%20Component%20Object%20Reference) (OtherActor :type Actor%20Object%20Reference) (OtherComp :type Primitive%20Component%20Object%20Reference) (OtherBodyIndex :type Integer) (bFromSweep :type Boolean) (SweepResult :type Hit%20Result%20Structure%20%28by%20ref%29))
  (if (and (== OtherActor (Variables|Default|GetPlayer)) (Variables|Default|GetDoorOpen))
    (Audio|PlaySoundatLocation "/Game/Sound/Desktops/MatrixShutdownSFX.MatrixShutdownSFX" (Transformation|GetWorldLocation (Variables|Default|GetTrigger)) "0, 0, 0" 1.0 1.0 0.0 0 0 0)
    (Utilities|FlowControl|Delay 1.5)
    (Game|OpenLevel(byName) "MatrixLevel")))

(event OnComponentBeginOverlap(DoorHandle)
  (params (OverlappedComponent :type Primitive%20Component%20Object%20Reference) (OtherActor :type Actor%20Object%20Reference) (OtherComp :type Primitive%20Component%20Object%20Reference) (OtherBodyIndex :type Integer) (bFromSweep :type Boolean) (SweepResult :type Hit%20Result%20Structure%20%28by%20ref%29))
  (if (== OtherActor (Variables|Default|GetPlayer))
    (Variables|Default|SetisInteracting true)))

(event OnComponentEndOverlap(DoorHandle)
  (params (OverlappedComponent :type Primitive%20Component%20Object%20Reference) (OtherActor :type Actor%20Object%20Reference) (OtherComp :type Primitive%20Component%20Object%20Reference) (OtherBodyIndex :type Integer))
  (if (== OtherActor (Variables|Default|GetPlayer))
    (Variables|Default|SetisInteracting false)))

(event EventBeginPlay
  (bind _outactors (Actor|GetAllActorsOfClass "/Game/VRTemplate/Blueprints/VRPawn.VRPawn_C"))
  (Variables|Default|SetPlayer (Utilities|Array|Get(acopy) _outactors))
  (Variables|Default|SetDoorOpen false))

(event EventTick
  (params (DeltaSeconds :type Float%20%28single-precision%29))
  (if (Variables|Default|GetDoorOpen)
    (Rendering|Components|Light|SetIntensity (Variables|Default|GetPointLight) 5e+03)))

(event EventTriggerPressed
  (if (Variables|Default|GetisInteracting)
    (Audio|PlaySoundatLocation "/Game/Sound/DoorHandleSFX.DoorHandleSFX" (Transformation|GetWorldLocation (Variables|Default|GetDoorHandle)) "0, 0, 0" 1.0 1.0 0.0 0 0 0)))

(fn ConstructionScript)