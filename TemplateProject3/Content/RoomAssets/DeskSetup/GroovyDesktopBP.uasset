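; Desktop PC prop in a VR room whose power button wakes "Groovy" and triggers the opening of the Matrix door.
; Trigger presses count only while the VR pawn overlaps the button.
; The first press powers off the PC, swapping the monitor material, fading the radio and starting a delayed sequence that switches the atmosphere cue's parameter, then opens the door.
; Later presses only play a click sound.
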(event OnComponentBeginOverlap(PowerButton)
  (params (OverlappedComponent :type Primitive%20Component%20Object%20Reference) (OtherActor :type Actor%20Object%20Reference) (OtherComp :type Primitive%20Component%20Object%20Reference) (OtherBodyIndex :type Integer) (bFromSweep :type Boolean) (SweepResult :type Hit%20Result%20Structure%20%28by%20ref%29))
  (if (== OtherActor (Variables|Default|GetPlayer))
    (Variables|Default|SetisInteracting true)))

(event OnComponentEndOverlap(PowerButton)
  (params (OverlappedComponent :type Primitive%20Component%20Object%20Reference) (OtherActor :type Actor%20Object%20Reference) (OtherComp :type Primitive%20Component%20Object%20Reference) (OtherBodyIndex :type Integer))
  (if (== OtherActor (Variables|Default|GetPlayer))
    (Variables|Default|SetisInteracting false)))

(event Custom|PCPowerOn
  (Audio|PlaySoundatLocation "/Game/Sound/Desktops/PowerOnCue.PowerOnCue" (Transformation|GetWorldLocation (Variables|Default|GetDesktopPCMesh)) "0, 0, 0" 1.0 1.0 0.0 0 0 0)
  (Rendering|Material|SetMaterial (Variables|/Game/RoomAssets/DeskSetup/Monitor/GroovyMonitorBP.GroovyMonitorBP_C|GetMonitor (Variables|Default|GetMonitorScreen)) 1 "/Game/RoomAssets/DeskSetup/Monitor/MonitorMaterialScreenOn.MonitorMaterialScreenOn"))

(event Custom|PCPowerOff
  (Audio|PlaySoundatLocation "/Game/Sound/Desktops/PowerOffGroovyCue.PowerOffGroovyCue" (Transformation|GetWorldLocation (Variables|Default|GetDesktopPCMesh)) "0, 0, 0" 1.0 1.0 0.0 0 0 0)
  (Rendering|Material|SetMaterial (Variables|/Game/RoomAssets/DeskSetup/Monitor/GroovyMonitorBP.GroovyMonitorBP_C|GetMonitor (Variables|Default|GetMonitorScreen)) 1 "/Game/RoomAssets/DeskSetup/Monitor/MonitorMaterialGroovy.MonitorMaterialGroovy")
  (Audio|Components|Audio|FadeOut (Variables|/Game/RoomAssets/Radio/RadioActor.RadioActor_C|GetRadio (Variables|Default|GetRadioActor)) 4.0 0.0 "Linear" :!class /Script/Engine.AudioComponent)
  (Utilities|FlowControl|Delay 9.0)
  (Effects|Components|ParticleSystem|SetIntParameter (Variables|Default|GetAtmosphereCue) "GroovyAwake" 1)
  (Utilities|FlowControl|Delay 12.0)
  (CallFunction|DoorAnimation))

(event Custom|DoorAnimation
  (Variables|Default|SetrunDoorAnim true)
  (Variables|Default|SetdoorOpen true)
  (Audio|PlaySoundatLocation "/Game/Sound/DoorOpenSFX.DoorOpenSFX" (Transformation|GetWorldLocation (Variables|/Script/Engine.Actor|GetRootComponent (Variables|Default|GetMatrixDoor))) "0, 0, 0" 1.0 1.0 0.0 0 0 0)
  (Utilities|FlowControl|Delay 2.0)
  (Variables|Default|SetrunDoorAnim false)
  (Variables|/Game/RoomAssets/Door/DoorBP.DoorBP_C|SetDoorOpen (Variables|Default|GetMatrixDoor) true))

(event EventBeginPlay
  (bind _outactors (Actor|GetAllActorsOfClass "/Game/VRTemplate/Blueprints/VRPawn.VRPawn_C"))
  (Variables|Default|SetPlayer (Utilities|Array|Get(acopy) _outactors))
  (Variables|Default|SetPowerStatus true)
  (Variables|Default|SetgroovyAsleep true)
  (Effects|Components|ParticleSystem|SetIntParameter (Variables|Default|GetAtmosphereCue) "GroovyAwake" 0)
  (Variables|Default|SetdoorOpen false)
  (Variables|Default|SetrunDoorAnim false))

(event EventTriggerPressed
  (if (Variables|Default|GetisInteracting)
    (bind _output_get (Variables|Default|SetPowerStatus (not (Variables|Default|GetPowerStatus))))
    (if (Variables|Default|GetgroovyAsleep)
      (if _output_get
        (CallFunction|PCPoweron)
        (else
          (CallFunction|PCPowerOff)
          (Variables|Default|SetgroovyAsleep false)))
      (else
        (Audio|PlaySoundatLocation "/Game/Sound/Desktops/PowerButtonClickSFX.PowerButtonClickSFX" (Transformation|GetWorldLocation (Variables|Default|GetDesktopPCMesh)) "0, 0, 0" 1.0 1.0 0.0 0 0 0)))))

(fn ConstructionScript)