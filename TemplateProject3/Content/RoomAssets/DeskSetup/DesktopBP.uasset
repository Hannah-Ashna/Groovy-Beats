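; Desktop computer prop for a VR room whose power button toggles its monitor on and off.
; It starts powered on and finds the VRPawn at BeginPlay, tracking when that pawn overlaps the PowerButton.
; TriggerPressed flips the power state only during that overlap.
; Tick sets the monitor's screen material on the MonitorScreen child to match the current state every frame.
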(event OnComponentBeginOverlap(PowerButton)
  (params (OverlappedComponent :type Primitive%20Component%20Object%20Reference) (OtherActor :type Actor%20Object%20Reference) (OtherComp :type Primitive%20Component%20Object%20Reference) (OtherBodyIndex :type Integer) (bFromSweep :type Boolean) (SweepResult :type Hit%20Result%20Structure%20%28by%20ref%29))
  (if (== OtherActor (Variables|Default|GetPlayer))
    (Variables|Default|SetisInteracting true)
    (Development|PrintString "PLAYER OVERLAP!")))

(event OnComponentEndOverlap(PowerButton)
  (params (OverlappedComponent :type Primitive%20Component%20Object%20Reference) (OtherActor :type Actor%20Object%20Reference) (OtherComp :type Primitive%20Component%20Object%20Reference) (OtherBodyIndex :type Integer))
  (if (== OtherActor (Variables|Default|GetPlayer))
    (Variables|Default|SetisInteracting false)))

(event EventTick
  (params (DeltaSeconds :type Float%20%28single-precision%29))
  (bind _monitorscreen (Variables|Default|GetMonitorScreen))
  (bind _monitor (Variables|/Game/RoomAssets/DeskSetup/Monitor/MonitorBP.MonitorBP_C|GetMonitor _monitorscreen))
  (if (Variables|Default|GetPowerStatus)
    (Rendering|Material|SetMaterial _monitor 1 "/Game/RoomAssets/DeskSetup/Monitor/MonitorMaterialScreenOn.MonitorMaterialScreenOn")
    (else
      (Rendering|Material|SetMaterial _monitor 1 "/Game/RoomAssets/DeskSetup/Monitor/MonitorMaterialScreenOff.MonitorMaterialScreenOff"))))

(event EventBeginPlay
  (bind _outactors (Actor|GetAllActorsOfClass "/Game/VRTemplate/Blueprints/VRPawn.VRPawn_C"))
  (Variables|Default|SetPlayer (Utilities|Array|Get(acopy) _outactors))
  (Variables|Default|SetPowerStatus true))

(event EventTriggerPressed
  (Development|PrintString "DESKTOP BP PRESSED")
  (if (Variables|Default|GetisInteracting)
    (Variables|Default|SetPowerStatus (not (Variables|Default|GetPowerStatus)))))

(fn ConstructionScript)